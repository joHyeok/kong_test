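; Player character with Enhanced Input movement, yaw turning, jumping and forward-only dash, plus two spheres that visualize leg bend.
; Movement follows control yaw, and move and turn values are stored with getters, turn for the Anim Blueprint.
; Dash plays or reverses a timeline that lerps max walk speed while moving forward.
; Each Tick, dot products of leg bone directions tint the spheres' dynamic materials from white (straight) to red (folded).
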(event Custom|InitInput
  ;[1 1 1] 입력 초기화
  ; 이동, 회전, 점프, 대시 4가지 입력 세팅
  (Utilities|IsValid (Variables|Default|GetAs%20BP%20PC%20Kong)
    (:Is%20Valid
      (Input|AddMappingContext (PlayerController|LocalPlayerSubsystems|GetEnhancedInputLocalPlayerSubsystem (Variables|Default|GetAs%20BP%20PC%20Kong)) "/Game/Blueprints/Input/IMC_Control.IMC_Control" 0 "(bIgnoreAllPressedKeysUntilRelease=True,bForceImmediately=False)"))))

(event Custom|SetSphereColor
  (bind _returnvalue (CallFunction|GetLogDot "thigh_r" "calf_r" "calf_r" "calf_twist_01_r"))
  (bind _returnvalue_2 (CallFunction|GetLogDot "thigh_l" "calf_l" "calf_l" "calf_twist_01_l"))
  (bind _returnvalue_3 (Math|Float|MapRangeClamped _returnvalue -1.0 1.0 0.0 1.0))
  (bind _returnvalue_4 (Math|Float|MapRangeClamped _returnvalue_2 -1.0 1.0 0.0 1.0))
  ;[1 1 1] 스피어 색 설정
  ; 많이 접힐수록 빨강 (1,0,0)
  ; 덜 접힐 수록 흰색 (1,1,1)
  ;;[1 1 1] 왼쪽 다리
  (Rendering|Material|SetVectorParameterValue (Variables|Default|GetLeftSphereMaterial) "Color" (Utilities|Struct|MakeLinearColor 1.0 _returnvalue_4 _returnvalue_4 1.0) :!class /Script/Engine.MaterialInstanceDynamic)
  ;;[1 1 1] 오른쪽 다리
  (Rendering|Material|SetVectorParameterValue (Variables|Default|GetRightSphereMaterial) "Color" (Utilities|Struct|MakeLinearColor 1.0 _returnvalue_3 _returnvalue_3 1.0) :!class /Script/Engine.MaterialInstanceDynamic))

(event Custom|InitSphereMaterial
  ;[1 1 1] 스피어 머티리얼 초기화
  (bind _returnvalue (Rendering|Material|CreateDynamicMaterialInstance (Variables|Default|GetLeft_Sphere) 0 "/Game/Art/MT/MI_Color.MI_Color" "None" :!class /Script/Engine.PrimitiveComponent))
  (Variables|Default|SetLeftSphereMaterial _returnvalue)
  (bind _returnvalue_2 (Rendering|Material|CreateDynamicMaterialInstance (Variables|Default|GetRight_Sphere) 0 "/Game/Art/MT/MI_Color.MI_Color" "None" :!class /Script/Engine.PrimitiveComponent))
  (Variables|Default|SetRightSphereMaterial _returnvalue_2))

(event Input|EnhancedActionEvents|EnhancedInputActionIA_Move
  (params (ActionValue :type Vector%202D%20Structure) (ElapsedSeconds :type Float%20%28double-precision%29) (TriggeredSeconds :type Float%20%28double-precision%29) (InputAction :type Input%20Action%20Object%20Reference :default "/Game/Blueprints/Input/IA_Move.IA_Move"))
  ;[1 1 1] Movement
  ; 폰 회전이 컨트롤러의 Yaw 값을 상속하고 있으므로 컨트롤러의 Yaw 값의 Forward Vector를 방향으로 잡고 Movement input 실행
  (:Triggered
    ;;[1 1 1] w를 눌렀는지 s를 눌렀는지 값 저장
    (Variables|Default|SetMoveForward (.x ActionValue))
    (Pawn|Input|AddMovementInput (Math|Vector|GetForwardVector (Math|Rotator|MakeRotator 0.0 0.0 (.yaw (Pawn|GetControlRotation :!class /Script/Engine.Pawn)))) (.x ActionValue) false)))

(event Input|EnhancedActionEvents|EnhancedInputActionIA_Jump
  (params (ActionValue :type Boolean) (ElapsedSeconds :type Float%20%28double-precision%29) (TriggeredSeconds :type Float%20%28double-precision%29) (InputAction :type Input%20Action%20Object%20Reference :default "/Game/Blueprints/Input/IA_Jump.IA_Jump"))
  ;[1 1 1] Jump
  ; 시작하고 완료될때 Jump 함수 실행
  (:Triggered
    (Character|Jump))
  (:Completed
    (Character|StopJumping)))

(event Input|EnhancedActionEvents|EnhancedInputActionIA_LeftShift
  (params (ActionValue :type Boolean) (ElapsedSeconds :type Float%20%28double-precision%29) (TriggeredSeconds :type Float%20%28double-precision%29) (InputAction :type Input%20Action%20Object%20Reference :default "/Game/Blueprints/Input/IA_LeftShift.IA_LeftShift"))
  ;[1 1 1] Dash
  ; 타임라인을 사용해 걷기 최대 속도를 0.8초 간격으로 300 ~ 600 사이를 상승, 하강한다
  (:Triggered
    ;;[1 1 1] 앞으로 움직이는 상태라면
    (if (CallFunction|IsForwardMove)
      (bind _0_1 (Timeline|AddMaxWalk Play)
        (:Update
          (Variables|/Script/Engine.CharacterMovementComponent|SetMaxWalkSpeed (Variables|Character|GetCharacterMovement) (Math|Float|Lerp 3e+02 6e+02 _0_1))))
      (else
        ;;[1 1 1] 움직이는 상태가 아니라면 최대 속도 300
        (Variables|/Script/Engine.CharacterMovementComponent|SetMaxWalkSpeed (Variables|Character|GetCharacterMovement) 3e+02 :!label _label))))
  (:Completed
    (if (CallFunction|IsForwardMove)
      (Timeline|AddMaxWalk Reverse)
      (else
        (goto _label)))))

(event Input|EnhancedActionEvents|EnhancedInputActionIA_Rotate
  (params (ActionValue :type Float%20%28double-precision%29) (ElapsedSeconds :type Float%20%28double-precision%29) (TriggeredSeconds :type Float%20%28double-precision%29) (InputAction :type Input%20Action%20Object%20Reference :default "/Game/Blueprints/Input/IA_Rotate.IA_Rotate"))
  ;[1 1 1] 회전
  ; 컨트롤러의 Yaw 값을 상속하고 있으므로 컨트롤러의 Yaw에 Input을 더해준다.
  ; Spring Arm은 움직이지 않도록 Yaw 상속을 꺼줬다.
  (:Triggered
    ;;[1 1 1] Anim Blueprint 에서 쓰기 위해 저장
    (Variables|Default|SetRotateValue ActionValue)
    (Pawn|Input|AddControllerYawInput (* ActionValue (Variables|Default|GetRotateSpeed))))
  (:Completed
    (Variables|Default|SetRotateValue 0.0)))

(event EventBeginPlay
  ;[1 1 1] BeginPlay
  ;;[1 1 1] PlayerController 가져오기
  (bind _asbp_pc_kong (Utilities|Casting|CastToBP_PC_Kong (Game|GetPlayerController 0)))
  (Variables|Default|SetAs%20BP%20PC%20Kong _asbp_pc_kong)
  ;;[1 1 1] 입력 세팅
  (CallFunction|InitInput)
  ;;[1 1 1] 스피어 머티리얼 초기화
  (CallFunction|InitSphereMaterial))

(event EventTick
  (params (DeltaSeconds :type Float%20%28single-precision%29))
  ;[1 1 1] Tick
  (CallFunction|SetSphereColor))

(fn ConstructionScript)

(fn IsForwardMove
  (return (and (CallFunction|IsMove) (> (Variables|Default|GetMoveForward) 0.0))))

(fn GetMoveForward
  (return (Variables|Default|GetMoveForward)))

(fn GetRotateValue
  (return (Variables|Default|GetRotateValue)))

(fn IsMove
  (return (> (Math|Vector|VectorLengthXY (Variables|/Script/Engine.MovementComponent|GetVelocity (Variables|Character|GetCharacterMovement))) 0.0)))

(fn GetLogDot
  (params (BoneNameFrom_1 :type Name) (BoneNameTo_1 :type Name) (BoneNameFrom_2 :type Name) (BoneNameTo_2 :type Name))
  (return (Math|Vector|DotProduct (Math|Vector|Normalize (Class|KismetAnimationLibrary|DirectionBetweenSockets (Variables|Character|GetMesh) BoneNameFrom_1 BoneNameTo_1)) (Math|Vector|Normalize (Class|KismetAnimationLibrary|DirectionBetweenSockets (Variables|Character|GetMesh) BoneNameFrom_2 BoneNameTo_2)))))